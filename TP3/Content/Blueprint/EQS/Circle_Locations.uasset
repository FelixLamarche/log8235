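; EQS context that supplies a set of locations around the player character tracked by the querier's SDTAIController.
; ProvideLocationsSet steps a pitch-rotated offset through a partial vertical arc around the player, starting a Visibility line trace at each point with no end point set.
; Hit impact points form the returned set, with debug printing and spheres after each hit.
; The EventGraph holds an unconnected copy of this logic.
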(fn ProvideLocationsSet
  (params (QuerierObject :type Object%20Object%20Reference) (QuerierActor :type Actor%20Object%20Reference))
  (bind _locations (Variables|Default|GetLocations))
  (Utilities|Array|Clear (Variables|Default|GetLocations))
  ;[1 1 1] Get registered agents size
  (for _index (range 0 9)
    (bind _assdtaicontroller (Utilities|Casting|CastToSDTAIController (AI|GetAIController QuerierActor)))
    (bind (_outhit _returnvalue) (Collision|LineTraceByChannel (+ (* (Math|Vector|RotateVector "1.000000, 0, 0" (Math|Rotator|MakeRotator 0.0 (* _index (/ 3.6e+02 15.0)) 0.0)) 5e+01) (Transformation|GetActorLocation (Variables|/Script/SoftDesignTraining.SDTAIController|GetplayerCharacter _assdtaicontroller))) "0, 0, 0" "TraceTypeQuery1" false (Utilities|Array|MakeArray 0 0) "None"))
    (if _returnvalue
      (Utilities|Array|Add _locations (.ImpactPoint (Collision|BreakHitResult _outhit)))
      (for _array_element _locations
        (Development|PrintString (Utilities|String|ToString(Vector) _array_element))
        (Rendering|Debug|DrawDebugSphere _array_element 2e+01 12 "(R=1.000000,G=0.059842,B=0.209745,A=1.000000)" 0.0))))
  (return (Variables|Default|GetLocations)))